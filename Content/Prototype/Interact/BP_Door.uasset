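; BP_Door is a double door that swings open and closed through interaction or pressure sources.
; A single timeline yaws the left and right pivots up to 90 degrees in opposite directions, playing to open, reversing to close, and flipping the closed flag when finished.
; Pressure sources increment or decrement a zero-clamped counter, so the door opens while any is active and closes when none remain.
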(event `/Game/Prototype/Interact/BI_Interaccions.OnInteracion`
  (bind _iscolsed (`self.IsColsed`))
  (if _iscolsed
    (bind (_direction _angleright _angleleft) (`Timeline|OpenCloseDoor` :!label _label)
      (:`Update`
        (`SceneComponent.K2_SetRelativeRotation` (`self.Pivot_Left`) (`KismetMathLibrary.MakeRotator` 0.0 0.0 (`KismetMathLibrary.Lerp` 0.0 90.0 _angleright)) false false)
        (`SceneComponent.K2_SetRelativeRotation` (`self.Pivot_Right`) (`KismetMathLibrary.MakeRotator` 0.0 0.0 (`KismetMathLibrary.Lerp` 0.0 -90.0 _angleleft)) false false))
      (:`Finished`
        (set `self.IsColsed` (not _iscolsed))))
    (else
      (goto _label :!via `Reverse`))))

(event `CloseDoor`
  (if (not (`self.IsColsed`))
    (goto _label :!via `Reverse`)))

(event `OpenDoor`
  (if (`self.IsColsed`)
    (goto _label)))

(fn `AddPresureSource`
  (bind _result (`/Engine/EditorBlueprintResources/StandardMacros.IncrementInt` (`self.ActivePressureCount`))
    (:`  `
      (set `self.ActivePressureCount` _result)
      (`self.UpdateDoorState`))))

(fn `RemovePressureSource`
  (bind _result (`/Engine/EditorBlueprintResources/StandardMacros.DecrementInt` (`self.ActivePressureCount`))
    (:`  `
      (set `self.ActivePressureCount` (`KismetMathLibrary.Max` _result))
      (`self.UpdateDoorState`))))

(fn `UpdateDoorState`
  (if (> (`self.ActivePressureCount`) 0)
    (`self.OpenDoor`)
    (else
      (`self.CloseDoor`))))

(fn `UserConstructionScript`
  (`parent.UserConstructionScript`))
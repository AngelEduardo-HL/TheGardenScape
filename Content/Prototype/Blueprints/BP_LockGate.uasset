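; Lock gate actor that ends the level once the player has enough keys and a referenced NPC has the flower.
; Overlapping its box as BP_ThirdPersonCharacter passes the character's key count to UpdateLocksVisual, which hides and disables collision on one of six locks per key held.
; If keys meet RequiredKeys and the valid NPCReference has HasFlower, it sets VictoryTriggered to block repeats and opens the victory level by name.
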(event `self.Box.OnComponentBeginOverlap`
  (params (OverlappedComponent :type "PrimitiveComponent Object Reference") (OtherActor :type "Actor Object Reference") (OtherComp :type "PrimitiveComponent Object Reference") (OtherBodyIndex :type Integer) (bFromSweep :type Boolean) (SweepResult :type "HitResult Structure (by ref)"))
  (bind _asbp_third_person_character (cast `/Game/ThirdPerson/Blueprints/BP_ThirdPersonCharacter` OtherActor))
  (if (not (`self.bVictoryTriggered`))
    (bind _currentkeys (`/Game/ThirdPerson/Blueprints/BP_ThirdPersonCharacter.CurrentKeys` _asbp_third_person_character))
    (`self.UpdateLocksVisual` _currentkeys)
    (if (>= _currentkeys (`self.RequiredKeys`))
      (`/Engine/EditorBlueprintResources/StandardMacros.IsValid` (`self.NPCReference`)
        (:`Is Valid`
          (if (`/Game/Prototype/AI/AI_NPC.bHasFlower` (`self.NPCReference`))
            (set `self.bVictoryTriggered` true)
            (`GameplayStatics.OpenLevel` (`self.VictoryLevelName`))))))))

(fn `UpdateLocksVisual`
  (params (CurrentKeys :type Integer))
  (if (>= CurrentKeys 1)
    (`SceneComponent.SetHiddenInGame` (`self.Lock1`) true false)
    (`PrimitiveComponent.SetCollisionEnabled` (`self.Lock1`) "NoCollision")
    (else
      (`SceneComponent.SetHiddenInGame` (`self.Lock1`) false false)
      (`PrimitiveComponent.SetCollisionEnabled` (`self.Lock1`) "QueryAndPhysics")))
  (if (>= (`local.CurrentKeys`) 2)
    (`SceneComponent.SetHiddenInGame` (`self.Lock2`) true false)
    (`PrimitiveComponent.SetCollisionEnabled` (`self.Lock2`) "NoCollision")
    (else
      (`SceneComponent.SetHiddenInGame` (`self.Lock2`) false false)
      (`PrimitiveComponent.SetCollisionEnabled` (`self.Lock2`) "QueryAndPhysics")))
  (if (>= (`local.CurrentKeys`) 3)
    (`SceneComponent.SetHiddenInGame` (`self.Lock3`) true false)
    (`PrimitiveComponent.SetCollisionEnabled` (`self.Lock3`) "NoCollision")
    (else
      (`SceneComponent.SetHiddenInGame` (`self.Lock3`) false false)
      (`PrimitiveComponent.SetCollisionEnabled` (`self.Lock3`) "QueryAndPhysics")))
  (if (>= (`local.CurrentKeys`) 4)
    (`SceneComponent.SetHiddenInGame` (`self.Lock4`) true false)
    (`PrimitiveComponent.SetCollisionEnabled` (`self.Lock4`) "NoCollision")
    (else
      (`SceneComponent.SetHiddenInGame` (`self.Lock4`) false false)
      (`PrimitiveComponent.SetCollisionEnabled` (`self.Lock4`) "QueryAndPhysics")))
  (if (>= (`local.CurrentKeys`) 5)
    (`SceneComponent.SetHiddenInGame` (`self.Lock5`) true false)
    (`PrimitiveComponent.SetCollisionEnabled` (`self.Lock5`) "NoCollision")
    (else
      (`SceneComponent.SetHiddenInGame` (`self.Lock5`) false false)
      (`PrimitiveComponent.SetCollisionEnabled` (`self.Lock5`) "QueryAndPhysics")))
  (if (>= (`local.CurrentKeys`) 6)
    (`SceneComponent.SetHiddenInGame` (`self.Lock6`) true false)
    (`PrimitiveComponent.SetCollisionEnabled` (`self.Lock6`) "NoCollision")
    (else
      (`SceneComponent.SetHiddenInGame` (`self.Lock6`) false false)
      (`PrimitiveComponent.SetCollisionEnabled` (`self.Lock6`) "QueryAndPhysics"))))

(fn `UserConstructionScript`
  (`parent.UserConstructionScript`))
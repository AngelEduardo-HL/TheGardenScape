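; BP_Lever is an interactable lever that toggles between up and down to control a linked door.
; Each interaction flips IsLeverDown, calling AddLeverSource on TargetDoor when pulled down and RemoveLeverSource when raised.
; A single animation serves both directions, played forward to lower and reversed from a set position to raise, with a 2D sound on every toggle.
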(event `/Game/Prototype/Interact/BI_Interaccions.OnInteracion`
  (if (`self.bIsLeverDown`)
    (`SkeletalMeshComponent.PlayAnimation` (`self.LeverMesh`) "/Game/Prototype/Assets/lever_Anim.lever_Anim" false)
    (`SkeletalMeshComponent.SetPlayRate` (`self.LeverMesh`) -1.0)
    (`SkeletalMeshComponent.SetPosition` (`self.LeverMesh`) 2.5 true)
    (set `self.bIsLeverDown` false)
    (`/Game/Prototype/Interact/BP_Door.RemoveLeverSource` (`self.TargetDoor`))
    (else
      (`SkeletalMeshComponent.PlayAnimation` (`self.LeverMesh`) "/Game/Prototype/Assets/lever_Anim.lever_Anim" false)
      (`SkeletalMeshComponent.SetPlayRate` (`self.LeverMesh`) 1.0)
      (`SkeletalMeshComponent.SetPosition` (`self.LeverMesh`) 0.0 true)
      (set `self.bIsLeverDown` true)
      (`/Game/Prototype/Interact/BP_Door.AddLeverSource` (`self.TargetDoor`))))
  (`GameplayStatics.PlaySound2D` "/Game/Prototype/Sounds/Lever_sfx.Lever_sfx" 1.0 1.0 0.0 null null))

(fn `UserConstructionScript`
  (`parent.UserConstructionScript`))